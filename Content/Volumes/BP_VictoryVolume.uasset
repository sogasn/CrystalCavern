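; BP_VictoryVolume is a level-exit volume that advances the game once the player has cleared the level of crystals.
; When the player pawn overlaps VinningCollision, it checks that no BP_Crystal actors remain in the world.
; It then finds the current map's index in the LevelNames array and opens the next level, or quits the game if that map is the last entry.
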(event `self.Vinning Collision.OnComponentBeginOverlap`
  (params (OverlappedComponent :type "PrimitiveComponent Object Reference") (OtherActor :type "Actor Object Reference") (OtherComp :type "PrimitiveComponent Object Reference") (OtherBodyIndex :type Integer) (bFromSweep :type Boolean) (SweepResult :type "HitResult Structure (by ref)"))
  (if (== OtherActor (`GameplayStatics.GetPlayerPawn` 0))
    (bind _outactors (`GameplayStatics.GetAllActorsOfClass` "/Game/Actors/Collectables/BP_Crystal.BP_Crystal_C"))
    (if (<= (`KismetArrayLibrary.Array_Length` _outactors) 0)
      (if (`self.Is Final Level`)
        (`KismetSystemLibrary.QuitGame` null "Quit")
        (else
          (`GameplayStatics.OpenLevel` (`|GetArrayItem` (`self.Level Names`) (+ (`self.Get Current Level Index`) 1))))))))

(fn `Get Current Level Index`
  (returns (ReturnValue :type Integer))
  (bind _returnvalue (`GameplayStatics.GetCurrentLevelName` true))
  (return (`KismetArrayLibrary.Array_Find` (`self.Level Names`) (`KismetStringLibrary.Conv_StringToName` _returnvalue))))

(fn `Is Final Level`
  (returns (ReturnValue :type Boolean))
  (return (== (`KismetArrayLibrary.Array_LastIndex` (`self.Level Names`)) (`self.Get Current Level Index`))))

(fn `UserConstructionScript`)