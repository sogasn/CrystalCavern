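; BP_Crystal is a collectable crystal actor that the player picks up by touching its collision volume.
; On overlap with the player pawn it caches its location, scale and light intensity, then plays the CollectTheCrystal timeline.
; Each update pulls the crystal toward the player's current position while shrinking it to zero and fading its light, and it destroys itself when the timeline finishes.
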(event `self.Player Collect Collision.OnComponentBeginOverlap`
  (params (OverlappedComponent :type "PrimitiveComponent Object Reference") (OtherActor :type "Actor Object Reference") (OtherComp :type "PrimitiveComponent Object Reference") (OtherBodyIndex :type Integer) (bFromSweep :type Boolean) (SweepResult :type "HitResult Structure (by ref)"))
  (if (== OtherActor (`GameplayStatics.GetPlayerPawn` 0))
    (`self.Set Starting Variables`)
    (bind (_direction _distance_to_player) (`Timeline|Collect the crystal`)
      (:`Update`
        (`self.Move To Player` _distance_to_player))
      (:`Finished`
        (`self.K2_DestroyActor`)))))

(fn `Move To Player`
  (params (Alpha :type "Float (double-precision)"))
  (`self.K2_SetActorLocation` (`KismetMathLibrary.VLerp` (`self.Lerp Start`) (`self.K2_GetActorLocation` (`GameplayStatics.GetPlayerPawn` 0)) Alpha))
  (`self.SetActorScale3D` (`KismetMathLibrary.VLerp` (`self.Starting Scale`) (0.0 0.0 0.0) Alpha))
  (`LightComponent.SetIntensity` (`self.Crystal Light`) (`KismetMathLibrary.Lerp` (`self.Starting Intensity`) 0.0 Alpha)))

(fn `Set Starting Variables`
  (set `self.Lerp Start` (`self.K2_GetActorLocation`))
  (set `self.Starting Scale` (`self.GetActorScale3D`))
  (set `self.Starting Intensity` (`LightComponentBase.Intensity` (`self.Crystal Light`))))

(fn `UserConstructionScript`)