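; BP_SpinningPlatform is an obstacle platform that repeatedly turns half a revolution around its yaw axis, pausing between turns.
; The SpinPlatform timeline drives SpinActor, which lerps from StartingRotation to 180 degrees of yaw beyond it along the shortest path.
; When the timeline finishes, it waits SpinningDelay, re-captures the current rotation as the new start and plays again, forming an endless loop from BeginPlay.
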(event `self.ReceiveBeginPlay`
  (set `self.Starting Rotation` (`self.K2_GetActorRotation`) :!label _label)
  (bind (_direction _spin) (`Timeline|Spin Platform` :!via `PlayFromStart`)
    (:`Update`
      (`self.Spin Actor` _spin))
    (:`Finished`
      (`KismetSystemLibrary.Delay` (`self.Spinning Delay`))
      (goto _label))))

(fn `Spin Actor`
  (params (Alpha :type "Float (double-precision)"))
  (`self.K2_SetActorRotation` (`KismetMathLibrary.RLerp` (`self.Starting Rotation`) (`KismetMathLibrary.MakeRotator` (.roll (`self.Starting Rotation`)) (.pitch (`self.Starting Rotation`)) (+ (.yaw (`self.Starting Rotation`)) 180.0)) Alpha true)))

(fn `UserConstructionScript`)