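; BP_Lift is a lift obstacle that moves its Cube back and forth between its starting relative location and LiftDestination.
; On BeginPlay it stores the start location, then a FlipFlop alternates between playing the Lift timeline forward and reversing it from the end.
; The timeline drives a position lerp without sweep, and its Finished output waits DelayDuration before re-entering the FlipFlop, forming an endless loop.
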(event `self.ReceiveBeginPlay`
  (set `self.Starting Location` (`SceneComponent.RelativeLocation` (`self.Cube`)))
  (`/Engine/EditorBlueprintResources/StandardMacros.FlipFlop` :!label _label
    (:`A`
      (bind (_direction _lift) (`Timeline|Lift` :!via `PlayFromStart` :!label _label_2)
        (:`Update`
          (`SceneComponent.K2_SetRelativeLocation` (`self.Cube`) (`KismetMathLibrary.VLerp` (`self.Starting Location`) (`self.Lift Destination`) _lift) false false))
        (:`Finished`
          (`KismetSystemLibrary.Delay` (`self.Delay Duration`))
          (goto _label))))
    (:`B`
      (goto _label_2 :!via `ReverseFromEnd`))))

(fn `UserConstructionScript`)