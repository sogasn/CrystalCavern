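; BP_Cannon is an obstacle actor that repeatedly fires projectiles on a timed loop from BeginPlay.
; After a fire-rate delay it spawns a BP_CannonProjecrile at the Arrow component's world transform, scaled by ProjectileScale.
; The CannonFire timeline then animates the cannon's relative Y location, and its Cannon Fired event loops back to the delay for the next shot.
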(event `self.ReceiveBeginPlay`
  (bind _arrow (`self.Arrow`))
  (`KismetSystemLibrary.Delay` (`self.Cannon Fire Rate`) :!label _label)
  (`|SpawnActorFromClass` "/Game/Actors/Projectiles/BP_CannonProjecrile.BP_CannonProjecrile_C" (`KismetMathLibrary.MakeTransform` (`SceneComponent.K2_GetComponentLocation` _arrow) (`SceneComponent.K2_GetComponentRotation` _arrow) (`KismetMathLibrary.Conv_DoubleToVector` (`self.Projectile Scale`))) "Undefined" "OverrideRootScale" null null)
  (bind (_direction _cannon_location) (`Timeline|Cannon Fire` :!via `PlayFromStart`)
    (:`Update`
      (`SceneComponent.K2_SetRelativeLocation` (`self.Cannon`) (`KismetMathLibrary.MakeVector` 0.0 _cannon_location) false false))
    (:`Cannon Fired`
      (goto _label))))

(fn `UserConstructionScript`)